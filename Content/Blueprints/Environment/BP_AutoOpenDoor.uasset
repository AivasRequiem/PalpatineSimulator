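; BP_AutoOpenDoor is an environment door that opens automatically when a PS_VRCharacter enters its trigger volume and closes when the character leaves.
; BeginPlay binds the OpenCollison begin and end overlap events.
; Each overlap swaps the open or close sound on one audio component and plays or reverses a timeline that slides the door along its relative Z axis.
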(event Custom|On%20OpenColision%20Begin%20Overlap
  (params (OverlappedComponent :type Primitive%20Component%20Object%20Reference) (OtherActor :type Actor%20Object%20Reference) (OtherComp :type Primitive%20Component%20Object%20Reference) (OtherBodyIndex :type Integer) (bFromSweep :type Boolean) (SweepResult :type Hit%20Result%20Structure%20%28by%20ref%29))
  (bind _door (Variables|Default|GetDoor))
  (bind _audio (Variables|Default|GetAudio))
  (bind _relativelocation (Variables|/Script/Engine.SceneComponent|GetRelativeLocation _door))
  (if (Class|GameplayStatics|ObjectIsA OtherActor "/Script/PalpatineSimulator.PS_VRCharacter")
    (Audio|Components|Audio|SetSound _audio (Variables|Default|GetOpenSound))
    (Audio|Components|Audio|Play _audio 0.0)
    (bind _openingdoor (Timeline|OpenTimeline Play)
      (:Update
        (Transformation|SetRelativeLocation _door (Math|Vector|MakeVector (.x _relativelocation) (.y _relativelocation) _openingdoor) false false)))))

(event Custom|On%20OpenColision%20End%20Overlap
  (params (OverlappedComponent :type Primitive%20Component%20Object%20Reference) (OtherActor :type Actor%20Object%20Reference) (OtherComp :type Primitive%20Component%20Object%20Reference) (OtherBodyIndex :type Integer))
  (bind _door (Variables|Default|GetDoor))
  (bind _audio (Variables|Default|GetAudio))
  (bind _relativelocation (Variables|/Script/Engine.SceneComponent|GetRelativeLocation _door))
  (if (Class|GameplayStatics|ObjectIsA OtherActor "/Script/PalpatineSimulator.PS_VRCharacter")
    (Audio|Components|Audio|SetSound _audio (Variables|Default|GetCloseSound))
    (Audio|Components|Audio|Play _audio 0.0)
    (bind _openingdoor (Timeline|OpenTimeline Reverse)
      (:Update
        (Transformation|SetRelativeLocation _door (Math|Vector|MakeVector (.x _relativelocation) (.y _relativelocation) _openingdoor) false false)))))

(event EventBeginPlay
  (bind _opencollison (Variables|Default|GetOpenCollison))
  (|CallParentFunction)
  (Collision|BindEventtoOnComponentBeginOverlap _opencollison (EventDispatchers|CreateEvent :!event Custom|On%20OpenColision%20Begin%20Overlap))
  (Collision|BindEventtoOnComponentEndOverlap _opencollison (EventDispatchers|CreateEvent :!event Custom|On%20OpenColision%20End%20Overlap)))

(fn ConstructionScript)