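; BP_LockedDoor is a door that stays locked until the player has deflected enough lasers and sliced enough objects.
; It binds to both PS_GameState objective events, and once both conditions hold it unlocks a single time, hides its lock indicator and queues an unlock sound through the game state.
; While locked, it suppresses the parent door's open-collision overlap handlers, so the inherited open behavior only runs after unlocking.
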(event Custom|TryUnlockDoor
  (bind _asps_game_state (Utilities|Casting|CastToPS_GameState (Game|GetGameState)))
  (if (and (Class|PSGameState|IsEnoughLasersDeflected _asps_game_state) (Class|PSGameState|IsEnoughObjectsSliced _asps_game_state))
    (Utilities|FlowControl|DoOnce false
      (:Completed
        (CallFunction|ChangeDoorState false)
        (bind _asps_game_state_2 (Utilities|Casting|CastToPS_GameState (Game|GetGameState)))
        (Class|PSGameState|AddSoundtoPlayQueue _asps_game_state_2 "/Game/Assets/Audio/Palpatine/DoorsUnlocked_Cue.DoorsUnlocked_Cue")))))

(event EventBeginPlay
  (|CallParentFunction)
  (bind _asps_game_state (Utilities|Casting|CastToPS_GameState (Game|GetGameState)))
  (EventDispatchers|AssignOnEnoughLasersDeflected _asps_game_state (delegate Custom|TryUnlockDoor))
  (EventDispatchers|BindEventtoOnEnoughObjectsSliced _asps_game_state (delegate Custom|TryUnlockDoor)))

(event EventOnOpenColisionBeginOverlap
  (params (OverlappedComponent :type Primitive%20Component%20Object%20Reference) (OtherActor :type Actor%20Object%20Reference) (OtherComp :type Primitive%20Component%20Object%20Reference) (OtherBodyIndex :type Integer) (bFromSweep :type Boolean) (SweepResult :type Hit%20Result%20Structure%20%28by%20ref%29))
  (if (not (Variables|Default|GetLocked))
    (|CallParentFunction OverlappedComponent OtherActor OtherComp OtherBodyIndex bFromSweep SweepResult)))

(event EventOnOpenColisionEndOverlap
  (params (OverlappedComponent :type Primitive%20Component%20Object%20Reference) (OtherActor :type Actor%20Object%20Reference) (OtherComp :type Primitive%20Component%20Object%20Reference) (OtherBodyIndex :type Integer))
  (if (not (Variables|Default|GetLocked))
    (|CallParentFunction OverlappedComponent OtherActor OtherComp OtherBodyIndex)))

(fn ConstructionScript
  (|CallParentFunction))

(fn ChangeDoorState
  (params (Lock :type Boolean))
  (bind _lockindicator (Variables|Default|GetLockIndicator))
  (bind _output_get (Variables|Default|SetLocked Lock))
  (if _output_get
    (Rendering|SetVisibility _lockindicator true false)
    (else
      (Rendering|SetVisibility _lockindicator false false))))