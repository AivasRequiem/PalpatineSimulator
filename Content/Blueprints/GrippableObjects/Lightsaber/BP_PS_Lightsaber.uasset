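; Grippable lightsaber Blueprint containing logic to slice procedural meshes with its blade, though no event triggers that logic, so it never runs.
; The unwired chain cuts a ProceduralMeshComponent along a plane at the TopBladeSocket, using the socket's Z axis as normal and the blade's material for the cap.
; The new half then gets physics simulation and a fixed velocity-change impulse.
; The construction script is empty.
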(fn ConstructionScript)