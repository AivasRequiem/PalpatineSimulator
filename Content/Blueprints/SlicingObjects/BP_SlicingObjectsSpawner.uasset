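; BP_SlicingObjectsSpawner is a spawner actor that launches BP_SlicingActor objects into the level.
; BeginPlay starts a looping two-second timer, presumably bound to SpawnSlicingActor, though the delegate's target is not shown.
; SpawnSlicingActor creates a scaled-down actor at the Cube component's location with random rotation, adjusting for collisions but always spawning.
; It then applies a random-strength, mass-dependent impulse to the SlicingMesh along the spawner's forward vector.
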(event EventBeginPlay
  (Utilities|Time|SetTimerbyEvent (EventDispatchers|CreateEvent :!event SpawnSlicingActor) 2.0 true))

(fn ConstructionScript)

(fn SpawnSlicingActor
  (bind _returnvalue (Game|SpawnActorfromClass "/Game/Blueprints/SlicingObjects/BP_SlicingActor.BP_SlicingActor_C" (Math|Transform|MakeTransform (Transformation|GetWorldLocation (Variables|Default|GetCube)) (Math|Random|RandomRotator true) "0.400000,0.400000,0.400000") "AdjustIfPossibleButAlwaysSpawn" "MultiplyWithRoot" 0 0))
  (Physics|AddImpulse (Variables|/Script/PalpatineSimulator.SlicingActor|GetSlicingMesh _returnvalue) (* (Transformation|GetActorForwardVector) (Math|Random|RandomFloatinRange 5e+03 1e+04)) "None" false))